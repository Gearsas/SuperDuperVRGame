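; Bullet casing actor for player guns that gets thrown out as a physics object when spawned.
; On BeginPlay the Case component receives a randomized velocity-change impulse along its negative right, forward and up axes, so mass is ignored and each casing flies slightly differently.
; The actor destroys itself after a fixed delay to clean up spent casings.
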(event `self.ReceiveBeginPlay`
  (bind _case (`self.Case`))
  (`PrimitiveComponent.AddImpulse` _case (+ (* (`SceneComponent.GetRightVector` _case) (`KismetMathLibrary.RandomFloatInRange` -100.0 -170.0)) (* (`SceneComponent.GetForwardVector` _case) (`KismetMathLibrary.RandomFloatInRange` -100.0 -170.0)) (* (`SceneComponent.GetUpVector` _case) (`KismetMathLibrary.RandomFloatInRange` -100.0 -170.0))) "None" true)
  (`KismetSystemLibrary.Delay` 30.0)
  (`self.K2_DestroyActor`))

(fn `UserConstructionScript`)