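; Weapon Blueprint for a Glock-style player gun, handling reload, ammo state and muzzle flash.
; Reload refills ammo after timed sounds, adding a slide animation when empty, while flags block shooting.
; Disconnected, never-executed shooting logic holds single-shot and burst paths that spawn bullets and casings from sockets.
; That logic calls the FlashyStuff macro, which briefly shows a light and flash mesh, then randomizes the mesh's rotation and scale.
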(event `Reload`
  (bind _returnvalue (`SceneComponent.GetSocketLocation` (`self.Gun`) "Muzzle"))
  (if (`self.IsReloading?`)
    _
    (elif (< (`self.GunAmmo`) (`self.MaxGunAmmo`))
      (if (== (`self.GunAmmo`) 0)
        (set `self.IsReloading?` true)
        (set `self.IsShooting?` true)
        (`GameplayStatics.PlaySoundAtLocation` "/Game/Player/Guns/Glock/Glock_sounds/GlockReload_Magazine.GlockReload_Magazine" _returnvalue (struct) 1.0 1.0 0.0 "/Game/Player/Guns/Glock/Glock_sounds/GLOCK.GLOCK" null null null)
        (`KismetSystemLibrary.Delay` 0.3)
        (`SkeletalMeshComponent.PlayAnimation` (`self.Gun`) "/Game/Player/Guns/Glock/Glock_Reload.Glock_Reload" false)
        (`GameplayStatics.PlaySoundAtLocation` "/Game/Player/Guns/Glock/Glock_sounds/GunReload_UpperThingy_Cue.GunReload_UpperThingy_Cue" _returnvalue (struct) 1.0 1.0 0.0 null null null null)
        (`KismetSystemLibrary.Delay` 0.2)
        (set `self.GunAmmo` (`self.MaxGunAmmo`))
        (set `self.IsReloading?` false)
        (set `self.IsShooting?` false)
        (else
          (set `self.IsReloading?` true)
          (set `self.IsShooting?` true)
          (`GameplayStatics.PlaySoundAtLocation` "/Game/Player/Guns/Glock/Glock_sounds/GlockReload_Magazine.GlockReload_Magazine" _returnvalue (struct) 1.0 1.0 0.0 null null null null)
          (`KismetSystemLibrary.Delay` 0.3)
          (set `self.GunAmmo` (`self.MaxGunAmmo`))
          (set `self.IsReloading?` false)
          (set `self.IsShooting?` false))))))

(fn `UserConstructionScript`)