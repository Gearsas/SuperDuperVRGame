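; Bullet actor that deals damage or pushes physics objects on impact, then destroys itself.
; On a capsule hit, a physics-simulating component receives an impulse at the bullet's location, scaled down from its velocity.
; Any other hit applies the bullet's Damage to the hit actor, with the instigator passed as damage causer.
; A delay started at BeginPlay destroys bullets that hit nothing within ten seconds.
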(event `self.ReceiveBeginPlay`
  (`KismetSystemLibrary.Delay` 10.0)
  (`self.K2_DestroyActor` :!label _label))

(event `self.Capsule.OnComponentHit`
  (params (HitComponent :type "PrimitiveComponent Object Reference") (OtherActor :type "Actor Object Reference") (OtherComp :type "PrimitiveComponent Object Reference") (NormalImpulse :type "Vector Structure") (Hit :type "HitResult Structure (by ref)"))
  (bind (_bblockinghit _binitialoverlap _time _distance _location _impactpoint _normal _impactnormal _physmat _hitactor _hitcomponent) (`GameplayStatics.BreakHitResult` Hit))
  (if (`SceneComponent.IsSimulatingPhysics` _hitcomponent "None")
    (`PrimitiveComponent.AddImpulseAtLocation` _hitcomponent (* (`self.GetVelocity`) 0.0001) (`self.K2_GetActorLocation`) "None")
    (goto _label)
    (else
      (`GameplayStatics.ApplyDamage` _hitactor (`self.Damage`) null (`self.GetInstigator`))
      (goto _label))))

(fn `UserConstructionScript`)