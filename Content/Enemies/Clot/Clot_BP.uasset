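; Clot enemy character that chases the VR player and ragdolls when killed.
; Pawn sensing starts an AI move toward the seen VRCharacter, re-issued shortly after each completed move.
; Any damage not caused by itself triggers death: it plays a hit sound, removes the capsule and sphere, simulates mesh physics and destroys the actor after a long delay.
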(event `self.PawnSensing.OnSeePawn`
  (params (Pawn :type "Pawn Object Reference"))
  ;[1 1 1] Player Sensing
  (bind _asvrcharacter (cast `/Game/Player/VRCharacter` Pawn))
  (`|AIMoveTo` self (0.0 0.0 0.0) _asvrcharacter 5.0 true :!label _label
    (:`then`
      (`KismetSystemLibrary.Delay` 0.2)
      (goto _label))))

(event `ragdoll`
  ;[1 1 1] After death character logic
  (`GameplayStatics.PlaySoundAtLocation` "/Game/Enemies/Clot/Clot_Sounds/getting_hit_1.getting_hit_1" (`SceneComponent.K2_GetComponentLocation` (`self.CapsuleComponent`)) (struct) 1.0 1.0 0.0 "/Game/Enemies/Clot/Clot_Sounds/hit_attenuation.hit_attenuation" null null null)
  (if (not (`self.IsDead?`))
    (set `self.IsDead?` true)
    (`ActorComponent.K2_DestroyComponent` (`self.CapsuleComponent`))
    (`PrimitiveComponent.SetSimulatePhysics` (`self.Mesh`) true)
    (`ActorComponent.K2_DestroyComponent` (`self.Sphere`))
    (`KismetSystemLibrary.Delay` 400.0)
    (`self.K2_DestroyActor`)))

(event `self.ReceiveAnyDamage`
  (params (Damage :type "Float (single-precision)") (DamageType :type "DamageType Object Reference") (InstigatedBy :type "Controller Object Reference") (DamageCauser :type "Actor Object Reference"))
  (if (!= self DamageCauser)
    (if (not (`self.IsDead?`))
      (`self.ragdoll`))))

(fn `UserConstructionScript`)